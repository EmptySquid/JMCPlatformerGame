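; BP_NPC is a platformer NPC that shows an interaction prompt while the player overlaps it and feeds timed dialogue to the player.
; It caches the player character on BeginPlay to filter overlaps and receive the dialogue text.
; UpdateDialogue writes the current line to the player, then re-calls itself after a fixed delay until the lines run out and clears the text.
; ResetDialogue restarts the sequence from the first line.
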(event `self.ReceiveBeginPlay`
  ; Player Reference
  (bind _asbp_third_person_character (cast `/Game/ThirdPerson/Blueprints/BP_ThirdPersonCharacter` (`GameplayStatics.GetPlayerPawn` 0)))
  (set `self.Player Reference` _asbp_third_person_character))

(event `self.ReceiveActorBeginOverlap`
  (params (OtherActor :type "Actor Object Reference"))
  ; Prompt Visibilty
  (if (== OtherActor (`self.Player Reference`))
    (`SceneComponent.SetVisibility` (`self.Interaction Prompt`) true false)))

(event `self.ReceiveActorEndOverlap`
  (params (OtherActor :type "Actor Object Reference"))
  ; Prompt Visibilty
  (if (== OtherActor (`self.Player Reference`))
    (`SceneComponent.SetVisibility` (`self.Interaction Prompt`) false false)))

(event `Update Dialogue`
  ; Update Dialogue
  (set `/Game/ThirdPerson/Blueprints/BP_ThirdPersonCharacter.Current Dialoge Text` (`|GetArrayItem` (`self.Dialogue Lines`) (`self.Current Dialogue Lines`)) (`self.Player Reference`))
  (set `self.Current Dialogue Lines` (+ (`self.Current Dialogue Lines`) 1))
  (`KismetSystemLibrary.Delay` 2.0)
  (if (!= (`self.Current Dialogue Lines`) (`KismetArrayLibrary.Array_Length` (`self.Dialogue Lines`)))
    (`self.Update Dialogue`)
    (else
      (set `/Game/ThirdPerson/Blueprints/BP_ThirdPersonCharacter.Current Dialoge Text` "" (`self.Player Reference`)))))

(event `Reset Dialogue`
  ; Reset Dialogue
  (set `self.Current Dialogue Lines` 0)
  (`self.Update Dialogue`))

(fn `UserConstructionScript`)