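; A vanishing platform actor that disappears after the player has stood on it for a set lifetime, then reappears.
; A trigger zone flags when the first player's pawn is on it, and Tick accumulates that time, resetting it when the player is off.
; On expiry it hides and disables collision, waits out an invisibility delay, then restores its starting transform, visibility and collision, with debug prints tracking overlaps and time.
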(event `self.ReceiveBeginPlay`
  (set `self.StartTransform` (`self.GetTransform`)))

(event `self.PlatformTriggerZone.OnComponentBeginOverlap`
  (params (OverlappedComponent :type "PrimitiveComponent Object Reference") (OtherActor :type "Actor Object Reference") (OtherComp :type "PrimitiveComponent Object Reference") (OtherBodyIndex :type Integer) (bFromSweep :type Boolean) (SweepResult :type "HitResult Structure (by ref)"))
  ; Player On/Off Platform
  (if (== OtherActor (`GameplayStatics.GetPlayerPawn` 0))
    (`|ExecutionSequence`
      (:`then_0`
        (`KismetSystemLibrary.PrintString` "PlayerOnPlatform"))
      (:`then_1`
        (set `self.IsPlayerOnPlatform` true)))))

(event `self.PlatformTriggerZone.OnComponentEndOverlap`
  (params (OverlappedComponent :type "PrimitiveComponent Object Reference") (OtherActor :type "Actor Object Reference") (OtherComp :type "PrimitiveComponent Object Reference") (OtherBodyIndex :type Integer))
  ; Player On/Off Platform
  (if (== OtherActor (`GameplayStatics.GetPlayerPawn` 0))
    (`|ExecutionSequence`
      (:`then_0`
        (`KismetSystemLibrary.PrintString` "PlayerOffPlatform"))
      (:`then_1`
        (set `self.IsPlayerOnPlatform` false)))))

(event `self.ReceiveTick`
  (params (DeltaSeconds :type "Float (single-precision)"))
  ; Set Time For Platform
  (if (`self.IsPlayerOnPlatform`)
    (bind _output_get (set `self.TimeOnPlatform` (+ DeltaSeconds (`self.TimeOnPlatform`))))
    (`KismetSystemLibrary.PrintString` (`KismetStringLibrary.Conv_DoubleToString` _output_get))
    ; Check Timer Life
    (if (>= (`self.TimeOnPlatform`) (`self.PlatformLifetime`))
      ; Hide and Disable Platform
      (`self.SetActorHiddenInGame` true)
      (`self.SetActorEnableCollision` false)
      (`KismetSystemLibrary.Delay` (`self.TimeInvisible`))
      (`self.ReturnToStart`))
    (else
      (set `self.TimeOnPlatform` 0.0))))

(event `ReturnToStart`
  (`SceneComponent.K2_SetWorldTransform` (`self.DefaultSceneRoot`) (`self.StartTransform`) false false)
  (set `self.TimeOnPlatform` 0.0)
  (`self.SetActorHiddenInGame` false)
  (`self.SetActorEnableCollision` true))

(fn `UserConstructionScript`)