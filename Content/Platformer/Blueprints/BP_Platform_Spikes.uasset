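; Platformer trap platform that thrusts five spike meshes up after the player steps on it.
; A box overlap from the player pawn starts a guarded cycle: wait PlatformLifetime, offset the spikes by SpikeLaunchDistance, wait again, then reverse the offset.
; The cycle completes even if the player leaves.
; Tick tracks and prints time on the platform, but its lifetime check triggers nothing.
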(event `self.ReceiveBeginPlay`)

(event `self.Box.OnComponentBeginOverlap`
  (params (OverlappedComponent :type "PrimitiveComponent Object Reference") (OtherActor :type "Actor Object Reference") (OtherComp :type "PrimitiveComponent Object Reference") (OtherBodyIndex :type Integer) (bFromSweep :type Boolean) (SweepResult :type "HitResult Structure (by ref)"))
  ; Player On/Off Platform
  (if (== OtherActor (`GameplayStatics.GetPlayerPawn` 0))
    (`|ExecutionSequence`
      (:`then_0`
        (`KismetSystemLibrary.PrintString` "PlayerOnPlatform")
        ; Spike Platform Detects Player
        (if (== (`self.SpikeInMotion`) false)
          (set `self.SpikeInMotion` true)
          (`KismetSystemLibrary.Delay` (`self.PlatformLifetime`))
          (`self.SpikeLaunch`)
          (`KismetSystemLibrary.Delay` (`self.PlatformLifetime`))
          (`self.ReturnToStart`)))
      (:`then_1`
        (set `self.IsPlayerOnPlatform` true)))))

(event `self.Box.OnComponentEndOverlap`
  (params (OverlappedComponent :type "PrimitiveComponent Object Reference") (OtherActor :type "Actor Object Reference") (OtherComp :type "PrimitiveComponent Object Reference") (OtherBodyIndex :type Integer))
  ; Player On/Off Platform
  (if (== OtherActor (`GameplayStatics.GetPlayerPawn` 0))
    (`|ExecutionSequence`
      (:`then_0`
        (`KismetSystemLibrary.PrintString` "PlayerOffPlatform"))
      (:`then_1`
        (set `self.IsPlayerOnPlatform` false)))))

(event `self.ReceiveTick`
  (params (DeltaSeconds :type "Float (single-precision)"))
  ; Set Time For Platform
  (if (`self.IsPlayerOnPlatform`)
    (bind _output_get (set `self.TimeOnPlatform` (+ DeltaSeconds (`self.TimeOnPlatform`))))
    (`KismetSystemLibrary.PrintString` (`KismetStringLibrary.Conv_DoubleToString` _output_get))
    ; Check Timer Life
    (if (>= (`self.TimeOnPlatform`) (`self.PlatformLifetime`))
      _)
    (else
      (set `self.TimeOnPlatform` 0.0))))

(event `SpikeLaunch`
  (bind _spikelaunchdistance (`self.SpikeLaunchDistance`))
  ; Spikes Go Up
  (`|ExecutionSequence`
    (:`then_0`
      (`SceneComponent.K2_AddWorldOffset` (`self.SM_Spike`) _spikelaunchdistance false false))
    (:`then_1`
      (`SceneComponent.K2_AddWorldOffset` (`self.SM_Spike1`) _spikelaunchdistance false false))
    (:`then_2`
      (`SceneComponent.K2_AddWorldOffset` (`self.SM_Spike2`) _spikelaunchdistance false false))
    (:`then_3`
      (`SceneComponent.K2_AddWorldOffset` (`self.SM_Spike3`) _spikelaunchdistance false false))
    (:`then_4`
      (`SceneComponent.K2_AddWorldOffset` (`self.SM_Spike4`) _spikelaunchdistance false false))))

(event `ReturnToStart`
  (bind _returnvalue (* (`self.SpikeLaunchDistance`) -1))
  ; Spikes Go Down
  (set `self.SpikeInMotion` false)
  (`|ExecutionSequence`
    (:`then_0`
      (`SceneComponent.K2_AddWorldOffset` (`self.SM_Spike`) _returnvalue false false))
    (:`then_1`
      (`SceneComponent.K2_AddWorldOffset` (`self.SM_Spike1`) _returnvalue false false))
    (:`then_2`
      (`SceneComponent.K2_AddWorldOffset` (`self.SM_Spike2`) _returnvalue false false))
    (:`then_3`
      (`SceneComponent.K2_AddWorldOffset` (`self.SM_Spike3`) _returnvalue false false))
    (:`then_4`
      (`SceneComponent.K2_AddWorldOffset` (`self.SM_Spike4`) _returnvalue false false))))

(fn `UserConstructionScript`)